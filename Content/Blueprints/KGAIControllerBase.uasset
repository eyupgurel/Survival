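; Base AI controller that makes its pawn hunt and melee player-controlled KGCharacterBase characters.
; A looping timer, rather than Tick, drives the logic: with no valid target, a sphere overlap around the controller actor's location picks the first player-controlled character found.
; The pawn moves to that target and tries a melee on arrival, or wanders to a random navigable point when none is found.
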(event `self.ReceiveBeginPlay`
  (`KismetSystemLibrary.K2_SetTimerDelegate` (delegate `ProcessAI`) 2.0 true))

(event `ProcessAI`
  (`self.Target`
    (:`then`
      (`|AIMoveTo` (`self.K2_GetPawn`) (0.0 0.0 0.0) (`self.Target`) :!label _label
        (:`OnSuccess`
          (bind _askgcharacter_base (cast `/Game/Blueprints/KGCharacterBase` (`self.K2_GetPawn`)))
          (`/Game/Blueprints/KGCharacterBase.TryMelee` _askgcharacter_base))))
    (:`else`
      (bind _outactors (`KismetSystemLibrary.SphereOverlapActors` (`self.K2_GetActorLocation`) 1000.0 (`|MakeArray` "ObjectTypeQuery3" :!type "EObjectTypeQuery Enum") "/Game/Blueprints/KGCharacterBase.KGCharacterBase_C" (`|MakeArray` (`self.K2_GetPawn`))))
      (for _array_element _outactors
        (bind _askgcharacter_base_2 (cast `/Game/Blueprints/KGCharacterBase` _array_element))
        (if (`self.IsPlayerController` (`Pawn.GetController` _askgcharacter_base_2))
          (set `self.Target` _askgcharacter_base_2)
          (break)))
      (`self.Target`
        (:`then`
          (goto _label))
        (:`else`
          (`self.Wander`))))))

(event `Wander`
  (bind _returnvalue (`self.K2_GetPawn`))
  (`/Engine/EditorBlueprintResources/StandardMacros.IsValid` _returnvalue
    (:`Is Valid`
      (`|AIMoveTo` _returnvalue (`NavigationSystem.K2_GetRandomLocationInNavigableRadius` (`self.K2_GetActorLocation` _returnvalue) 2000.0) null 10.0))))

(fn `UserConstructionScript`)